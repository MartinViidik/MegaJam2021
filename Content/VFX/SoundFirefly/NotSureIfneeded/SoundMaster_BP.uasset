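; SoundMaster is an audio-reactive Blueprint that plays a soundtrack and scales a sphere to its frequency content.
; The audio component's playback-percent event is converted to elapsed seconds using the track's duration.
; That time samples normalized channel-0 bands from offline Constant-Q (Audio Synesthesia) data.
; Each band calls Play on one shared timeline, whose update lerps sphere scale from unit size toward the tripled band value.
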(event `self.ReceiveBeginPlay`
  (bind _soundtrack (`self.Soundtrack`))
  (`AudioComponent.SetSound` (`self.Audio`) _soundtrack)
  (set `self.Duration` (`SoundBase.Duration` _soundtrack))
  (add `AudioComponent.OnAudioPlaybackPercent` (`self.Audio`) (`|CreateDelegate` :!event `PlaybackChange`))
  (`AudioComponent.Play` (`self.Audio`) 0.0))

(event `PlaybackChange`
  (params (PlayingSoundWave :type "SoundWave Object Reference") (PlaybackPercent :type "Float (double-precision)"))
  (set `self.Played Time` (* PlaybackPercent (`self.Duration`)))
  (for _array_element (`ConstantQNRT.GetNormalizedChannelConstantQAtTime` (`self.Constant_REf`) (`self.Played Time`) 0)
    (bind (_direction _newtrack_0) (`Timeline|Timeline_0`)
      (:`Update`
        (`SceneComponent.SetWorldScale3D` (`self.Sphere`) (`KismetMathLibrary.VLerp` (1.0 1.0 1.0) (* (`KismetMathLibrary.Conv_DoubleToVector` _array_element) 3.0) _newtrack_0))))))

(fn `UserConstructionScript`)