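; Tile controller that builds a grid of child actor components in the world from its construction script.
; ConstructWorld runs nested loops over XValue and YValue, adding one component per cell at the transform requested from GetSpawnTransform.
; GetSpawnTransform contains staggered-grid math, spacing cells by XSpacing and YSpacing and shifting odd X columns by Offset in Y, though that expression appears unconnected.
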(event `self.ReceiveBeginPlay`)

(fn `ConstructWorld`
  (for _index (range (+ (`self.XValue`) 1))
    (for _index_2 (range (+ (`self.YValue`) 1))
      (`AddComponent|NODE_AddChildActorComponent-0` :`RelativeTransform` (`self.GetSpawnTransform` _index_2 _index)))))

(fn `UserConstructionScript`
  (`self.ConstructWorld`))