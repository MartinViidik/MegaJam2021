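; BP_Tile is a damageable world tile that shows a floating health bar when hurt and defers death handling to its parent.
; BeginPlay caches the WBP_HealthBar and makes its widget component invisible.
; TakeDamage, when health differs from max, shows the widget, updates its fill and sets a three-second timer to HideWidget.
; HideWidget uses Hidden In Game, which the show path's SetVisibility never resets.
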(event `/Game/Blueprints/Interfaces/BPI_Health.HandleDeath`
  (`parent.HandleDeath`))

(event `self.ReceiveBeginPlay`
  (`parent.ReceiveBeginPlay`)
  (bind _aswbp_health_bar (cast `/Game/Blueprints/Widgets/WBP_HealthBar` (`WidgetComponent.GetUserWidgetObject` (`self.Widget`))))
  (set `self.HealthBar` _aswbp_health_bar)
  (`SceneComponent.SetVisibility` (`self.Widget`) false false))

(event `HideWidget`
  (`SceneComponent.SetHiddenInGame` (`self.Widget`) true false)
  (`KismetSystemLibrary.K2_ClearAndInvalidateTimerHandle` (stale `/Game/Blueprints/Interfaces/BPI_Health.TakeDamage` _returnvalue)))

(event `/Game/Blueprints/Interfaces/BPI_Health.TakeDamage`
  (bind _widget (`self.Widget`))
  (bind _bp_healthcomponent (`self.BP_HealthComponent`))
  (bind _health (`/Game/Blueprints/Components/BP_HealthComponent.Health` _bp_healthcomponent))
  (bind _maxhealthh (`/Game/Blueprints/Components/BP_HealthComponent.MaxHealthh` _bp_healthcomponent))
  (if (!= _health _maxhealthh)
    (if (not (`SceneComponent.IsVisible` _widget))
      (`SceneComponent.SetVisibility` _widget true false))
    (`/Game/Blueprints/Widgets/WBP_HealthBar.SetFillAmount` (`self.HealthBar`) (`KismetMathLibrary.Conv_IntToDouble` _health) (`KismetMathLibrary.Conv_IntToDouble` _maxhealthh))
    (bind _returnvalue (`KismetSystemLibrary.K2_SetTimerDelegate` (delegate `HideWidget`) 3.0))))

(fn `UserConstructionScript`
  (`parent.UserConstructionScript`))