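; BP_TileBase is a world tile that hosts one building and can be destroyed.
; ConstructBuilding spawns the requested class at BuildingRoot after a short delay, and the tile's health component takes that building's base health.
; Death destroys any building, decrements the game mode's tile count and spawns grass VFX.
; SetHexVisibility toggles mesh and building widget, while player-proximity reveal logic is left disconnected.
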(event `/Game/Blueprints/Interfaces/BPI_Tile.SetHexVisibility`
  (params (Hidden :type Boolean))
  (`SceneComponent.SetHiddenInGame` (`self.StaticMesh`) Hidden false)
  (bind _buildingref (`self.BuildingRef`)
    (:`then`
      (`/Game/Blueprints/Buildings/BP_BuildingBase.SetWidgetVisibility` _buildingref (not Hidden)))
    (:`else`)))

(event `/Game/Blueprints/Interfaces/BPI_Tile.ConstructBuilding`
  (params (TargetClass :type "/Game/Blueprints/Buildings/BP_BuildingBase Class Reference"))
  (`KismetSystemLibrary.Delay` 1.25)
  (`self.SpawnBuilding` TargetClass))

(event `/Game/Blueprints/Interfaces/BPI_Health.HandleDeath`
  (bind _buildingref (`self.BuildingRef`)
    (:`then`
      (`/Game/Blueprints/Buildings/BP_BuildingBase.DestroyBuilding` _buildingref)
      (set `self.BuildingRef` null))
    (:`else`
      _))
  (`/Game/Blueprints/Misc/Game/BP_GameMode.DecrementTiles` (`/Game/Blueprints/Functions/BP_Library.GetGameModeActor`))
  ;[1 1 1] SpawnGrassOnTileDeath
  (bind _returnvalue (`NiagaraFunctionLibrary.SpawnSystemAtLocation` "/Game/VFX/GrowingGrass/VFX_GrowinGrass.VFX_GrowinGrass" (`SceneComponent.K2_GetComponentLocation` (`self.StaticMesh`))))
  (`PrimitiveComponent.SetCastShadow` _returnvalue true)
  (`self.K2_DestroyActor`))

(event `/Game/Blueprints/Interfaces/BPI_Tile.Upgrade`
  (bind _buildingref (`self.BuildingRef`))
  (`/Engine/EditorBlueprintResources/StandardMacros.IsValid` _buildingref
    (:`Is Valid`
      (`/Game/Blueprints/Buildings/BP_BuildingBase.UpgradeBuilding` _buildingref))))

(event `self.Sphere.OnComponentBeginOverlap`
  (params (OverlappedComponent :type "PrimitiveComponent Object Reference") (OtherActor :type "Actor Object Reference") (OtherComp :type "PrimitiveComponent Object Reference") (OtherBodyIndex :type Integer) (bFromSweep :type Boolean) (SweepResult :type "HitResult Structure (by ref)"))
  ;[1 1 1] Unhide on Player Collision
)

(event `self.Sphere.OnComponentEndOverlap`
  (params (OverlappedComponent :type "PrimitiveComponent Object Reference") (OtherActor :type "Actor Object Reference") (OtherComp :type "PrimitiveComponent Object Reference") (OtherBodyIndex :type Integer))
  ;[1 1 1] Hide
)

(event `/Game/Blueprints/Interfaces/BPI_Health.TakeDamage`
  (`/Game/Blueprints/Components/BP_CharacterAudio.PlayHitSound` (`self.BP_CharacterAudio`)))

(fn `SpawnBuilding`
  (params (TargetBuilding :type "/Game/Blueprints/Buildings/BP_BuildingBase Class Reference"))
  (bind _bp_healthcomponent (`self.BP_HealthComponent`))
  (`self.BuildingRef`
    (:`then`)
    (:`else`
      (bind _returnvalue (`|SpawnActorFromClass` TargetBuilding (`SceneComponent.K2_GetComponentToWorld` (`self.BuildingRoot`)) "AlwaysSpawn" "OverrideRootScale" null null))
      (bind _output_get (set `self.BuildingRef` _returnvalue))
      (`self.SetOwner` _output_get self)
      (bind _basehealth (`/Game/Blueprints/Buildings/BP_BuildingBase.BaseHealth` _output_get))
      (set `/Game/Blueprints/Components/BP_HealthComponent.MaxHealthh` _basehealth _bp_healthcomponent)
      (set `/Game/Blueprints/Components/BP_HealthComponent.Health` _basehealth _bp_healthcomponent))))

(fn `UserConstructionScript`
  (`PrimitiveComponent.SetCollisionObjectType` (`self.StaticMesh`) "ECC_GameTraceChannel1"))