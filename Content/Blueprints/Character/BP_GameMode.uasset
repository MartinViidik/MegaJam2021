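; BP_GameMode is a Game Mode Blueprint that tracks the current money and handles building purchases on tiles.
; ConstructBuilding compares a value from the building's class defaults, used as its cost, against CurrentMoney.
; If affordable, it sends ConstructBuildingMessage to the tile, then deducts the truncated cost through UpdateMoney.
; ReturnCurrentMoney exposes the balance, and UpdateMoney applies a signed modifier without any clamping.
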(fn `ConstructBuilding`
  (params (Building :type "/Game/Blueprints/Buildings/BP_BuildingBase Class Reference") (Tile :type "Object Object Reference"))
  (bind _buildingcost (defaults `Object` Building))
  (if (<= _buildingcost (`self.CurrentMoney`))
    (message `/Game/Blueprints/Interfaces/BPI_Tile.ConstructBuilding` Tile Building)
    (`self.UpdateMoney` (`KismetMathLibrary.FTrunc` (* _buildingcost -1.0)))))

(fn `ReturnCurrentMoney`
  (returns (Money :type Integer))
  (return (`self.CurrentMoney`)))

(fn `UpdateMoney`
  (params (Modifier :type Integer))
  (set `self.CurrentMoney` (+ (`self.CurrentMoney`) Modifier)))

(fn `UserConstructionScript`)