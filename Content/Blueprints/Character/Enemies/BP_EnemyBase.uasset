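; BP_EnemyBase is an enemy character whose max health and attack damage scale with the game mode's wave number.
; On BeginPlay it caches its BP_AIController, hides its widget and sets those stats on its health and attack components.
; Attack passes the controller's current target to the attack component and plays a sound.
; HandleDeath reports the kill to the game mode, spawns a score popup, plays death audio and destroys the actor.
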(event `self.ReceiveBeginPlay`
  (bind _asbp_aicontroller (cast `/Game/Blueprints/Character/Enemies/BP_AIController` (`AIBlueprintHelperLibrary.GetAIController` self)))
  (set `self.ControllerRef` _asbp_aicontroller)
  (`SceneComponent.SetVisibility` (`self.Widget`) false false)
  (set `/Game/Blueprints/Components/BP_HealthComponent.MaxHealthh` (`KismetMathLibrary.FTrunc` (/ (* (`/Game/Blueprints/Misc/Game/BP_GameMode.WaveNr` (`/Game/Blueprints/Functions/BP_Library.GetGameModeActor`)) 10.0) 2.0)) (`self.BP_HealthComponent`))
  (set `/Game/Blueprints/Components/BP_AttackComponent.Damage` (`KismetMathLibrary.FTrunc` (/ (* (`/Game/Blueprints/Misc/Game/BP_GameMode.WaveNr` (`/Game/Blueprints/Functions/BP_Library.GetGameModeActor`)) 10.0) 6.5)) (`self.BP_AttackComponent`)))

(event `/Game/Blueprints/Interfaces/BPI_Health.HandleDeath`
  (`/Game/Blueprints/Misc/Game/BP_GameMode.IncrementKills` (`/Game/Blueprints/Functions/BP_Library.GetGameModeActor`) self)
  (bind _returnvalue (`|SpawnActorFromClass` "/Game/Blueprints/Misc/Game/BP_ScoreUpdate.BP_ScoreUpdate_C" (`self.GetTransform`) "Undefined" "OverrideRootScale" null null))
  (`/Game/Blueprints/Misc/Game/BP_ScoreUpdate.UpdateText` _returnvalue 10 true)
  (`/Game/Blueprints/Components/BP_CharacterAudio.PlayDeathSound` (`self.BP_CharacterAudio`))
  (`self.K2_DestroyActor`))

(event `Attack`
  (bind _asbp_aicontroller (cast `/Game/Blueprints/Character/Enemies/BP_AIController` (`AIBlueprintHelperLibrary.GetAIController` self)))
  (`/Game/Blueprints/Components/BP_AttackComponent.AttackTarget` (`self.BP_AttackComponent`) (`/Game/Blueprints/Character/Enemies/BP_AIController.CurrentTarget` _asbp_aicontroller))
  (`/Game/Blueprints/Components/BP_CharacterAudio.PlayAttackSound` (`self.BP_CharacterAudio`)))

(fn `UserConstructionScript`)