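; BP_MeleeEnemy is a melee enemy child Blueprint that adds health bar feedback on top of its parent class.
; On BeginPlay it casts its widget component's user widget to WBP_HealthBar and caches it.
; TakeDamage reveals the hidden widget and sets the bar's fill from the health component's current and max health.
; Attack and the construction script only call the parent, while Tick and overlap events are disabled.
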(event `self.ReceiveBeginPlay`
  (`parent.ReceiveBeginPlay`)
  (bind _aswbp_health_bar (cast `/Game/Blueprints/Widgets/WBP_HealthBar` (`WidgetComponent.GetUserWidgetObject` (`self.Widget`))))
  (set `self.HealthBar` _aswbp_health_bar))

(event `self.Attack`
  (`parent.Attack`))

(event `/Game/Blueprints/Interfaces/BPI_Health.TakeDamage`
  (bind _bp_healthcomponent (`self.BP_HealthComponent`))
  (if (not (`SceneComponent.IsVisible` (`self.Widget`)))
    (`SceneComponent.SetVisibility` (`self.Widget`) true false)
    (`SceneComponent.SetVisibility` (`self.Widget`) true false))
  (`/Game/Blueprints/Widgets/WBP_HealthBar.SetFillAmount` (`self.HealthBar`) (`KismetMathLibrary.Conv_IntToDouble` (`/Game/Blueprints/Components/BP_HealthComponent.Health` _bp_healthcomponent)) (`KismetMathLibrary.Conv_IntToDouble` (`/Game/Blueprints/Components/BP_HealthComponent.MaxHealthh` _bp_healthcomponent))))

(fn `UserConstructionScript`
  (`parent.UserConstructionScript`))