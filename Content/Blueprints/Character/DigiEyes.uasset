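; DigiEyes is a character's digital eye display that shows emotions by swapping the TextureParam texture on a dynamic material instance created in the Construction Script.
; Angry, sad and hurt events show their texture for a given duration, then restore idle, while death stays permanently.
; A RunningCustomEyes flag marks active expressions.
; A Timer timeline holds randomised single and double blinks gated by that flag, but nothing starts it.
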(event `self.ReceiveBeginPlay`
  (set `self.RunningCustomEyes?` false))

(event `AngryEyes`
  (params (`Emoji Duration` :type "Float (double-precision)"))
  ;[0 0 0 0] Angry
  (set `self.RunningCustomEyes?` true)
  (`MaterialInstanceDynamic.SetTextureParameterValue` (`self.DigiEyes_MI`) "TextureParam" "/Game/Textures/Character/Mad.Mad")
  (`KismetSystemLibrary.Delay` `Emoji Duration`)
  (set `self.RunningCustomEyes?` false)
  (`MaterialInstanceDynamic.SetTextureParameterValue` (`self.DigiEyes_MI`) "TextureParam" "/Game/Textures/Character/Idle.Idle"))

(event `SadEyes`
  (params (`Emoji Duration` :type "Float (double-precision)"))
  ;[0 0 0 0] Sad
  (set `self.RunningCustomEyes?` true)
  (`MaterialInstanceDynamic.SetTextureParameterValue` (`self.DigiEyes_MI`) "TextureParam" "/Game/Textures/Character/Sad.Sad")
  (`KismetSystemLibrary.Delay` `Emoji Duration`)
  (set `self.RunningCustomEyes?` false)
  (`MaterialInstanceDynamic.SetTextureParameterValue` (`self.DigiEyes_MI`) "TextureParam" "/Game/Textures/Character/Idle.Idle"))

(event `Hurt`
  (params (`Emoji Duration` :type "Float (double-precision)"))
  ;[0 0 0 0] Alternate Hurt
  (set `self.RunningCustomEyes?` true)
  (`MaterialInstanceDynamic.SetTextureParameterValue` (`self.DigiEyes_MI`) "TextureParam" "/Game/Textures/Character/Hurt.Hurt")
  (`KismetSystemLibrary.Delay` `Emoji Duration`)
  (set `self.RunningCustomEyes?` false)
  (`MaterialInstanceDynamic.SetTextureParameterValue` (`self.DigiEyes_MI`) "TextureParam" "/Game/Textures/Character/Idle.Idle"))

(event `Death`
  ;[0 0 0 0] Dead
  (set `self.RunningCustomEyes?` true)
  (`MaterialInstanceDynamic.SetTextureParameterValue` (`self.DigiEyes_MI`) "TextureParam" "/Game/Textures/Character/Dead.Dead"))

(fn `UserConstructionScript`
  (bind _returnvalue (`PrimitiveComponent.CreateDynamicMaterialInstance` (`self.DigitalEyes_01`) 0 "/Game/Materials/DigitalEyesMat_Inst.DigitalEyesMat_Inst" "None"))
  (set `self.DigiEyes_MI` _returnvalue))