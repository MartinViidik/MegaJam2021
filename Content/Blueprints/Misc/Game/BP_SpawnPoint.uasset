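; BP_SpawnPoint is a spawn area actor that supplies random positions inside a configurable box volume.
; The construction script sizes the Box component from the XExtent, YExtent and ZExtent variables.
; GetRandomPoint returns a random point within that extent, centered on the root component's world location.
; The sampling is axis-aligned and uses the unscaled extent, so actor rotation and scale do not affect it.
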(fn `GetRandomPoint`
  (returns (ReturnValue :type "Vector Structure"))
  (return (`KismetMathLibrary.RandomPointInBoundingBox` (`SceneComponent.K2_GetComponentLocation` (`self.DefaultSceneRoot`)) (`BoxComponent.BoxExtent` (`self.Box`)))))

(fn `UserConstructionScript`
  (`BoxComponent.SetBoxExtent` (`self.Box`) (`KismetMathLibrary.MakeVector` (`self.XExtent`) (`self.YExtent`) (`self.ZExtent`)) true))