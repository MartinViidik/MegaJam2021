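; Game mode for a wave-based base defense game, owning money, building purchases, the main UI, pause and game over.
; The first building purchase starts growing waves of timer-spawned AI at random spawn points, with a 60-second timeout that clears leftovers and forces the next wave.
; Kills and cleared waves pay money, each purchase raises that building type's cost, and losing every tile ends the game.
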(event `SpawnEnemy`
  (if (> (`self.SpawnedEnemies`) (`self.EnemyCount`))
    (`self.StopTimer`)
    (else
      (bind _returnvalue (`AIBlueprintHelperLibrary.SpawnAIFromClass` (`|GetArrayItem` (`self.Tier1Enemies`)) "/Game/Blueprints/Character/Enemies/BT_BehaviourTree.BT_BehaviourTree" (`/Game/Blueprints/Misc/Game/BP_SpawnPoint.GetRandomPoint` (`KismetArrayLibrary.Array_Random` (`self.SpawnPoints`))) (struct) true null))
      (`/Engine/EditorBlueprintResources/StandardMacros.IncrementInt` (`self.SpawnedEnemies`)
        (:`  `
          (`KismetArrayLibrary.Array_Add` (`self.SpawnedActors`) _returnvalue))))))

(event `IncrementKills`
  (params (Pawn :type "Pawn Object Reference"))
  (bind _enemycount (`self.EnemyCount`))
  (`KismetArrayLibrary.Array_RemoveItem` (`self.SpawnedActors`) Pawn)
  (bind _result (`/Engine/EditorBlueprintResources/StandardMacros.IncrementInt` (`self.KilledEnemies`))
    (:`  `
      (`KismetSystemLibrary.PrintString` (`KismetStringLibrary.Conv_IntToString` _enemycount))
      (`self.UpdateMoney` 10)
      (if (== _result _enemycount)
        (`self.WaveOver`)))))

(event `StartEnemyTimer`
  (params (SpawnCooldown :type "Float (double-precision)"))
  (bind _returnvalue (`KismetSystemLibrary.K2_SetTimerDelegate` (`|CreateDelegate` :!event `SpawnEnemy`) SpawnCooldown true))
  (set `self.SpawnTimer` _returnvalue))

(event `StopTimer`
  (`KismetSystemLibrary.K2_ClearAndInvalidateTimerHandle` (`self.SpawnTimer`)))

(event `WaveOver`
  (`/Game/Blueprints/Widgets/WBP_GameUI.PlayWaveOverAnim` (`self.GameUI`))
  (`KismetSystemLibrary.K2_SetTimerDelegate` (`|CreateDelegate` :!event `StartNewWave`) 7.0)
  (`self.UpdateMoney` (* (`self.WaveNr`) 30)))

(event `StartNewWave`
  (bind _resettimer (`self.ResetTimer`))
  (if (`KismetSystemLibrary.K2_IsValidTimerHandle` _resettimer)
    (`KismetSystemLibrary.K2_ClearAndInvalidateTimerHandle` _resettimer))
  (set `self.EnemyCount` (+ (`self.EnemyCount`) 5))
  (bind _result (`/Engine/EditorBlueprintResources/StandardMacros.IncrementInt` (`self.WaveNr`))
    (:`  `
      (`self.StartEnemyTimer` (`self.EnemyCooldown`))
      (`/Game/Blueprints/Widgets/WBP_GameUI.PlayWaveStartAnim` (`self.GameUI`) _result)
      (bind _returnvalue (`KismetSystemLibrary.K2_SetTimerDelegate` (delegate `ResetWave`) 60.0))
      (set `self.ResetTimer` _returnvalue))))

(event `ResetWave`
  (for _array_element (`self.SpawnedActors`)
    (`self.K2_DestroyActor` _array_element))
  (`KismetArrayLibrary.Array_Clear` (`self.SpawnedActors`))
  (`self.StartNewWave`))

(event `self.ReceiveBeginPlay`
  (bind _gameui (`self.GameUI`))
  (bind _outactors (`GameplayStatics.GetAllActorsOfClass` "/Game/Blueprints/Misc/Game/BP_SpawnPoint.BP_SpawnPoint_C"))
  (set `self.SpawnPoints` _outactors)
  (bind _outactors_2 (`GameplayStatics.GetAllActorsOfClass` "/Game/Blueprints/World/BP_TileBase.BP_TileBase_C"))
  (set `self.AmountOfTiles` (`KismetArrayLibrary.Array_Length` _outactors_2))
  (bind _returnvalue (`|CreateWidget` "/Game/Blueprints/Widgets/WBP_GameUI.WBP_GameUI_C" (`GameplayStatics.GetPlayerController` 0)))
  (bind _output_get (set `self.GameUI` _returnvalue))
  (`UserWidget.AddToViewport` _output_get 0)
  (`/Game/Blueprints/Widgets/WBP_GameUI.UpdateResources` _gameui (`self.CurrentMoney`))
  (`WidgetBlueprintLibrary.SetInputMode_GameOnly` (`GameplayStatics.GetPlayerController` 0))
  (`PlayerCameraManager.StartCameraFade` :`self` (`GameplayStatics.GetPlayerCameraManager` 0) :`FromAlpha` 1.0 :`Duration` 1.0 :`bShouldFadeAudio` true :`bHoldWhenFinished` true)
  (`/Game/Blueprints/Widgets/WBP_GameUI.TEXTANIM` _gameui))

(event `DecrementTiles`
  (bind _result (`/Engine/EditorBlueprintResources/StandardMacros.DecrementInt` (`self.AmountOfTiles`))
    (:`  `
      (bind _output_get (set `self.AmountOfTiles` _result))
      (if (<= _output_get 0)
        (`self.GameOver`)))))

(event `GameOver`
  (`WidgetBlueprintLibrary.SetInputMode_UIOnlyEx` (`GameplayStatics.GetPlayerController` 0) null)
  (`Widget.RemoveFromParent` (`self.GameUI`))
  (`PlayerCameraManager.StartCameraFade` :`self` (`GameplayStatics.GetPlayerCameraManager` 0) :`ToAlpha` 1.0 :`Duration` 1.0 :`bShouldFadeAudio` true :`bHoldWhenFinished` true)
  (`KismetSystemLibrary.K2_SetTimerDelegate` (`|CreateDelegate` :!event `ReloadLevel`) 3.0))

(event `RemoveUI`
  (`Widget.RemoveFromParent` (`self.GameUI`)))

(event `ReloadLevel`
  (bind _returnvalue (`GameplayStatics.GetCurrentLevelName` true))
  (`GameplayStatics.OpenLevel` (`KismetStringLibrary.Conv_StringToName` _returnvalue)))

(fn `ConstructBuilding`
  (params (Tile :type "Object Object Reference") (BuildingEnum :type "/Game/Misc/Enums/EN_Buildings Enum" :default "NewEnumerator0"))
  (locals (ClassRef :type "/Game/Blueprints/Buildings/BP_BuildingBase Class Reference") (Cost :type Integer) (TileRef :type "Object Object Reference") (EnumRef :type "/Game/Misc/Enums/EN_Buildings Enum" :default "NewEnumerator0"))
  (set `local.EnumRef` BuildingEnum)
  (set `local.TileRef` Tile)
  (switch `/Game/Misc/Enums/EN_Buildings` BuildingEnum
    (:`NewEnumerator0`
      (set `local.ClassRef` "/Game/Blueprints/Buildings/BP_Building2_HitScan.BP_Building2_HitScan_C")
      (set `local.Cost` (`self.TurretCost`)))
    (:`NewEnumerator1`
      (set `local.ClassRef` "/Game/Blueprints/Buildings/BP_Building1.BP_Building1_C")
      (set `local.Cost` (`self.ResourceCost`)))
    (:`NewEnumerator2`
      (set `local.ClassRef` "/Game/Blueprints/Buildings/BP_Building3.BP_Building3_C")
      (set `local.Cost` (`self.HealingCost`))))
  (if (<= (`local.Cost`) (`self.CurrentMoney`))
    (message `/Game/Blueprints/Interfaces/BPI_Tile.ConstructBuilding` (`local.TileRef`) (`local.ClassRef`))
    (bind _asbp_character (cast `/Game/Blueprints/Character/BP_Character` (`GameplayStatics.GetPlayerCharacter` 0)))
    (set `/Game/Meshes/Character/BP_CharacterAnim.Build` true (`/Game/Blueprints/Character/BP_Character.As BP Character Anim` _asbp_character))
    (`GameplayStatics.PlaySoundAtLocation` "/Game/Sound/Buildings/button_pressed_on_arm_Cue.button_pressed_on_arm_Cue" (`self.K2_GetActorLocation` _asbp_character) (struct) 1.0 1.0 0.0 null null _asbp_character)
    (`self.UpdateMoney` (`KismetMathLibrary.FTrunc` (* (`local.Cost`) -1.0)))
    (`self.UpdateBuildingCounts` (`local.EnumRef`) (`local.Cost`))
    ;[1 1 1] Handle game start
    (bind _result (`/Engine/EditorBlueprintResources/StandardMacros.IncrementInt` (`self.BuildingCount`))
      (:`  `
        (if (== _result 1)
          (`self.StartNewWave`))))
    (else
      (bind _asbp_character_2 (cast `/Game/Blueprints/Character/BP_Character` (`GameplayStatics.GetPlayerCharacter` 0)))
      (set `/Game/Meshes/Character/BP_CharacterAnim.Build` false (`/Game/Blueprints/Character/BP_Character.As BP Character Anim` _asbp_character_2)))))

(fn `ReturnCurrentMoney`
  (returns (Money :type Integer))
  (return (`self.CurrentMoney`)))

(fn `ReturnSpawnedActors`
  (returns (SpawnedActors :type "Array of Pawn Object Reference"))
  (return (`self.SpawnedActors`)))

(fn `SetGamePauseState`
  (bind _returnvalue (`GameplayStatics.GetPlayerController` 0))
  (`Widget.SetVisibility` (`/Game/Blueprints/Widgets/WBP_GameUI.PausePanel` (`self.GameUI`)) "Visible")
  (`WidgetBlueprintLibrary.SetInputMode_GameAndUIEx` _returnvalue null)
  (set `PlayerController.bShowMouseCursor` true _returnvalue)
  (`GameplayStatics.SetGamePaused` true))

(fn `SetGameResumeState`
  (bind _returnvalue (`GameplayStatics.GetPlayerController` 0))
  (`GameplayStatics.SetGamePaused` false)
  (`Widget.SetVisibility` (`/Game/Blueprints/Widgets/WBP_GameUI.PausePanel` (`self.GameUI`)) "Hidden")
  (`WidgetBlueprintLibrary.SetInputMode_GameOnly` _returnvalue)
  (set `PlayerController.bShowMouseCursor` false _returnvalue))

(fn `UpdateBuildingCounts`
  (params (BuildingType :type "/Game/Misc/Enums/EN_Buildings Enum" :default "NewEnumerator0") (CurrentCost :type Integer))
  (locals (CostRef :type Integer) (TypeRef :type "/Game/Misc/Enums/EN_Buildings Enum" :default "NewEnumerator0"))
  (bind (_returnvalue _returnvalue2) (`self.NewMacro_0`))
  (bind (_returnvalue_2 _returnvalue2_2) (`self.NewMacro_0`))
  (bind (_returnvalue_3 _returnvalue2_3) (`self.NewMacro_0`))
  (set `local.CostRef` CurrentCost)
  (bind _output_get (set `local.TypeRef` BuildingType))
  (switch `/Game/Misc/Enums/EN_Buildings` _output_get
    (:`NewEnumerator0`
      (`/Engine/EditorBlueprintResources/StandardMacros.IncrementInt` (`self.TurretCount`)
        (:`  `
          (set `self.TurretCost` _returnvalue_2)
          (`/Game/Blueprints/Widgets/WBP_GameUI.UpdateBuildingUI` (`self.GameUI`) (`local.TypeRef`) _returnvalue2_2))))
    (:`NewEnumerator1`
      (`/Engine/EditorBlueprintResources/StandardMacros.IncrementInt` (`self.ResourceCount`)
        (:`  `
          (set `self.ResourceCost` _returnvalue_3)
          (`/Game/Blueprints/Widgets/WBP_GameUI.UpdateBuildingUI` (`self.GameUI`) (`local.TypeRef`) _returnvalue2_3))))
    (:`NewEnumerator2`
      (`/Engine/EditorBlueprintResources/StandardMacros.IncrementInt` (`self.HealingCount`)
        (:`  `
          (set `self.HealingCost` _returnvalue)
          (`/Game/Blueprints/Widgets/WBP_GameUI.UpdateBuildingUI` (`self.GameUI`) (`local.TypeRef`) _returnvalue2))))))

(fn `UpdateMoney`
  (params (Modifier :type Integer))
  (bind _output_get (set `self.CurrentMoney` (+ (`self.CurrentMoney`) Modifier)))
  (`/Game/Blueprints/Widgets/WBP_GameUI.UpdateResources` (`self.GameUI`) _output_get))

(fn `UpdatePlayerHealthUI`
  (params (CurrentHealth :type Integer))
  (`/Game/Blueprints/Widgets/WBP_GameUI.UpdatePlayerHealth` (`self.GameUI`) CurrentHealth))

(fn `UserConstructionScript`)