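; BP_ScoreUpdate is a short-lived floating text actor that shows score changes through a WBP_ScoreUpdate widget component.
; On BeginPlay it nudges itself by a small random offset, then a timeline moves the widget along world Z each update and destroys the actor when finished.
; UpdateText and SimpleSetText forward either a number and increment or a modifier to the widget.
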(event `self.ReceiveBeginPlay`
  (`self.K2_AddActorLocalOffset` (`KismetMathLibrary.MakeVector` (`KismetMathLibrary.RandomFloatInRange` -10.0 10.0) (`KismetMathLibrary.RandomFloatInRange` -10.0 10.0) (`KismetMathLibrary.RandomFloatInRange` -10.0 10.0)))
  (bind (_direction _newtrack_0) (`Timeline|Timeline_0`)
    (:`Update`
      (`SceneComponent.K2_SetWorldLocation` (`self.Widget`) (+ (`SceneComponent.K2_GetComponentLocation` (`self.Widget`)) (`KismetMathLibrary.MakeVector` 0.0 0.0 _newtrack_0)) false false))
    (:`Finished`
      (`self.K2_DestroyActor`))))

(event `UpdateText`
  (params (Number :type Integer) (Increment :type Boolean))
  (bind _aswbp_score_update (cast `/Game/Blueprints/Widgets/WBP_ScoreUpdate` (`WidgetComponent.GetUserWidgetObject` (`self.Widget`))))
  (`/Game/Blueprints/Widgets/WBP_ScoreUpdate.SetScoreText` _aswbp_score_update Number Increment))

(event `SimpleSetText`
  (params (Modifier :type Integer))
  (bind _aswbp_score_update (cast `/Game/Blueprints/Widgets/WBP_ScoreUpdate` (`WidgetComponent.GetUserWidgetObject` (`self.Widget`))))
  (`/Game/Blueprints/Widgets/WBP_ScoreUpdate.SimpleSetText` _aswbp_score_update Modifier))

(fn `UserConstructionScript`)