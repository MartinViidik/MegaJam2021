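; Game mode for the intro screen that shows an intro widget and moves on to the main game map.
; On BeginPlay it creates WBP_Intro, adds it to the viewport and sets game-and-UI input.
; Tick polls the Space key, and a DoOnce fades the widget out, waits briefly, then opens GameMap4.
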(event `self.ReceiveBeginPlay`
  (bind _returnvalue (`|CreateWidget` "/Game/Blueprints/Widgets/WBP_Intro.WBP_Intro_C"))
  (`UserWidget.AddToViewport` _returnvalue 0)
  (`WidgetBlueprintLibrary.SetInputMode_GameAndUIEx` (`GameplayStatics.GetPlayerController` 0) null))

(event `self.ReceiveTick`
  (params (DeltaSeconds :type "Float (single-precision)"))
  (if (`PlayerController.IsInputKeyDown` (`GameplayStatics.GetPlayerController` 0) "SpaceBar")
    (`/Engine/EditorBlueprintResources/StandardMacros.DoOnce` false
      (:`Completed`
        (`/Game/Blueprints/Widgets/WBP_Intro.FadeOut` (stale `self.ReceiveBeginPlay` _returnvalue))
        (`KismetSystemLibrary.Delay` 2.0)
        (`GameplayStatics.OpenLevel` "GameMap4")))))

(fn `UserConstructionScript`)