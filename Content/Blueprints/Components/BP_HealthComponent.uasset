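; BP_HealthComponent is a component that tracks its owning actor's health and signals when it runs out.
; BeginPlay stores the starting Health as the maximum, and UpdateHealth adds a signed modifier, clamps the result between zero and that maximum and prints it.
; At zero, HealthEmpty calls HandleDeathMessage on the owner, leaving the death response to that actor.
; The HealthGone function is an empty stub.
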(event `self.ReceiveBeginPlay`
  (set `self.MaxHealthh` (`self.Health`)))

(event `UpdateHealth`
  (params (Modifier :type Integer))
  (bind _output_get (set `self.Health` (`KismetMathLibrary.Clamp` (+ (`self.Health`) Modifier) 0 (`self.MaxHealthh`))))
  (`KismetSystemLibrary.PrintString` (`KismetStringLibrary.Concat_StrStr` "Actor:" (`KismetSystemLibrary.GetDisplayName` (`self.GetOwner`)) " Current Health:" (`KismetStringLibrary.Conv_IntToString` _output_get)))
  (if (<= (`self.Health`) 0)
    (`self.HealthEmpty`)))

(event `HealthEmpty`
  (message `/Game/Blueprints/Interfaces/BPI_Health.HandleDeath` (`self.GetOwner`)))

(fn `HealthGone`)