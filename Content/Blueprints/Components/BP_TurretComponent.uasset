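; Turret component that picks a target from the game mode's spawned actors and computes the rotation to face it.
; OptimisedSearch keeps the nearest actor within a distance cap and enables component and owner ticking, while BeginPlay starts a looping timer.
; Tick computes LookAtRotation from the owner's "Rotate"-tagged mesh to the target.
; An older random sphere-overlap search for enemies remains unconnected, and IsTargetValid reports target validity.
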(event `OptimisedSearch`
  (for _array_element (`/Game/Blueprints/Misc/Game/BP_GameMode.SpawnedActors` (`/Game/Blueprints/Functions/BP_Library.GetGameModeActor`))
    (bind _returnvalue (`Actor.GetDistanceTo` _array_element (`self.GetOwner`)))
    (if (< _returnvalue (`self.Distance`))
      (set `self.Distance` _returnvalue)
      (bind _output_get (set `self.TargetActor` _array_element))
      (`KismetSystemLibrary.PrintString` (`KismetSystemLibrary.GetDisplayName` _output_get))))
  (set `self.Distance` 10000.0)
  (`self.SetComponentTickEnabled` true)
  (`Actor.SetActorTickEnabled` (`self.GetOwner`) true))

(event `self.ReceiveBeginPlay`
  (bind _returnvalue (`KismetSystemLibrary.K2_SetTimerDelegate` (`|CreateDelegate` :!event `OptimisedSearch`) 0.75 true))
  (set `self.TimerRef` _returnvalue)
  (set `self.NewVar_0` (`|GetArrayItem` (`Actor.GetComponentsByTag` (`self.GetOwner`) "/Script/Engine.StaticMeshComponent" "Rotate"))))

(event `SearchForTargets`)

(event `self.ReceiveTick`
  (params (DeltaSeconds :type "Float (single-precision)"))
  (`/Engine/EditorBlueprintResources/StandardMacros.IsValid` (`self.TargetActor`)
    (:`Is Valid`
      (set `self.LookAtRotation` (`KismetMathLibrary.FindLookAtRotation` (`SceneComponent.K2_GetComponentLocation` (`self.NewVar_0`)) (`Actor.K2_GetActorLocation` (`self.TargetActor`)))))))

(fn `IsTargetValid`
  (returns (NewParam :type Boolean))
  (return (`KismetSystemLibrary.IsValid` (`self.TargetActor`))))