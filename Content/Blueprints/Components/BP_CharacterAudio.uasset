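; Character audio component that handles footstep and attack sounds for its owner.
; SetSurfaceType caches the surface type from a hit material, and FootstepSound switches on it, currently only printing debug text for grass or default steps.
; PlayAttackSound plays AttackSound at the GetOwnerLocation result, though that function's owner-location lookup is left unconnected.
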(event `FootstepSound`
  (switch `EPhysicalSurface` (`self.SurfaceType`)
    (:`SurfaceType_Default`
      (`KismetSystemLibrary.PrintString` "DEFAULT step"))
    (:`SurfaceType1`
      (`KismetSystemLibrary.PrintString` "GRASS step"))))

(event `SetSurfaceType`
  (params (HitMaterial :type "PhysicalMaterial Object Reference"))
  (set `self.SurfaceType` (`PhysicalMaterial.SurfaceType` HitMaterial)))

(event `PlayAttackSound`
  (`GameplayStatics.PlaySoundAtLocation` (`self.AttackSound`) (`self.GetOwnerLocation`) (struct) 1.0 1.0 0.0 null null null))