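; Actor component that gives its owner radial and single-target attacks, dealing damage through BP_HealthComponent.
; AttackRadial runs a fixed-radius sphere overlap around the owner, excluding it, and subtracts Damage from every hit actor that has a health component.
; A CanAttack flag and one-shot timer enforce the Cooldown between radial attacks.
; AttackTarget damages the given actor directly, bypassing the cooldown and validity check.
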(event `SetCanAttack`
  (set `self.CanAttack` true))

(event `ResetCooldown`
  (`KismetSystemLibrary.K2_SetTimerDelegate` (delegate `SetCanAttack`) (`self.Cooldown`)))

(event `AttackRadial`
  (params (`[0]` :type "EObjectTypeQuery Enum" :default "ObjectTypeQuery1"))
  (if (`self.CanAttack`)
    (set `self.CanAttack` false)
    (`self.ResetCooldown`)
    (bind _outactors (`KismetSystemLibrary.SphereOverlapActors` (`Actor.K2_GetActorLocation` (`self.GetOwner`)) 150.0 (`|MakeArray` `[0]`) null (`|MakeArray` (`self.GetOwner`))))
    (for _array_element _outactors
      (bind _returnvalue (`Actor.GetComponentByClass` _array_element "/Game/Blueprints/Components/BP_HealthComponent.BP_HealthComponent_C"))
      (`/Engine/EditorBlueprintResources/StandardMacros.IsValid` _returnvalue
        (:`Is Valid`
          (`/Game/Blueprints/Components/BP_HealthComponent.UpdateHealth` _returnvalue (* (`self.Damage`) -1)))))))

(event `AttackTarget`
  (params (TargetActor :type "Actor Object Reference"))
  (`/Game/Blueprints/Components/BP_HealthComponent.UpdateHealth` (`Actor.GetComponentByClass` TargetActor "/Game/Blueprints/Components/BP_HealthComponent.BP_HealthComponent_C") (* (`self.Damage`) -1)))