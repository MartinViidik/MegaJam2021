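; Healing component that restores health to non-enemy actors around its owner.
; HealInRadius sphere-overlaps at the owner's location, skips BP_EnemyBase actors and adds HealRate through each damaged actor's BP_HealthComponent, without checking that the component exists.
; Each heal calls RetractFlowers, which forwards to the owner only if it is a BP_Building3.
; The ActorClassFilter input is not passed to the overlap.
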(event `HealInRadius`
  (params (ObjectTypes :type "Array of EObjectTypeQuery Enum (by ref)") (ActorClassFilter :type "Object Class Reference"))
  (bind _outactors (`KismetSystemLibrary.SphereOverlapActors` (`SceneComponent.K2_GetComponentLocation` (`Actor.RootComponent` (`self.GetOwner`))) (`self.HealRadius`) ObjectTypes))
  (for _array_element _outactors
    (cast `/Game/Blueprints/Character/Enemies/BP_EnemyBase` _array_element
      (:`CastFailed`
        (bind _returnvalue (`Actor.GetComponentByClass` _array_element "/Game/Blueprints/Components/BP_HealthComponent.BP_HealthComponent_C"))
        (if (!= (`/Game/Blueprints/Components/BP_HealthComponent.Health` _returnvalue) (`/Game/Blueprints/Components/BP_HealthComponent.MaxHealthh` _returnvalue))
          (`/Game/Blueprints/Components/BP_HealthComponent.UpdateHealth` _returnvalue (`self.HealRate`))
          (`self.RetractFlowers`))))))

(event `RetractFlowers`
  (bind _asbp_building_3 (cast `/Game/Blueprints/Buildings/BP_Building3` (`self.GetOwner`)))
  (`/Game/Blueprints/Buildings/BP_Building3.RetractFlowers` _asbp_building_3))