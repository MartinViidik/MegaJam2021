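; BP_SpeedModifier is a component that switches its owner's walk speed between slow, regular and fast states.
; On BeginPlay it caches the owner's CharacterMovementComponent and applies the base speed.
; The SetSpeed event maps the requested state to a MaxWalkSpeed value, but only while the current speed is non-zero, so a speed of zero stays in place.
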(event `self.ReceiveBeginPlay`
  (bind _output_get (set `self.MoveComponentRef` (`Actor.GetComponentByClass` (`self.GetOwner`) "/Script/Engine.CharacterMovementComponent")))
  (set `CharacterMovementComponent.MaxWalkSpeed` (`self.BaseSpeed`) _output_get))

(event `SetSpeed`
  (params (SpeedState :type "/Game/Misc/Enums/EN_SpeedState Enum" :default "NewEnumerator0"))
  (if (!= (`CharacterMovementComponent.MaxWalkSpeed` (`self.MoveComponentRef`)) 0.0)
    (set `CharacterMovementComponent.MaxWalkSpeed` (select `/Game/Misc/Enums/EN_SpeedState` SpeedState :`NewEnumerator0` (`self.SlowdownSpeed`) :`NewEnumerator1` (`self.BaseSpeed`) :`NewEnumerator2` (`self.FastSpeed`)) (`self.MoveComponentRef`))))