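; BP_Building1 is a resource tower building that earns money for the game mode on a looping timer, with upgrades raising the payout.
; It extends a parent building's events, pausing the timer while in a backpack, resuming it when restored and clearing it on destruction.
; Timelines slide the shovel into place, then loop its pitch rotation, alongside startup and loop sounds, a sped-up particle system and the upgrade widget flag.
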(event `ShovelRotation`
  (bind (_direction _pitch) (`Timeline|RotateTimeline` :!via `PlayFromStart`)
    (:`Update`
      (`SceneComponent.K2_SetRelativeRotation` (`self.RotatingShovelComponent`) (`KismetMathLibrary.MakeRotator` 0.0 _pitch) false false))
    (:`Finished`
      (`self.ShovelRotation`))))

(event `self.ReceiveBeginPlay`
  (`parent.ReceiveBeginPlay`)
  (bind _asbp_game_mode (cast `/Game/Blueprints/Misc/Game/BP_GameMode` (`GameplayStatics.GetGameMode`)))
  (set `self.GameModeRef` _asbp_game_mode)
  (bind _returnvalue (`KismetSystemLibrary.K2_SetTimerDelegate` (`|CreateDelegate` :!event `AddResources`) (`self.ResourceDelay`) true))
  (set `self.TimerRef` _returnvalue))

(event `AddResources`
  (`/Game/Blueprints/Misc/Game/BP_GameMode.UpdateMoney` (`self.GameModeRef`) (`self.ResourceAdd`)))

(event `self.BuildingDestroyed`
  (if (`KismetSystemLibrary.K2_IsValidTimerHandle` (`self.TimerRef`))
    (`KismetSystemLibrary.K2_ClearAndInvalidateTimerHandle` (`self.TimerRef`)))
  (`parent.BuildingDestroyed`))

(event `self.UpgradeBuilding`
  (set `self.ResourceAdd` (+ (`self.ResourceAdd`) 25))
  (`parent.UpgradeBuilding`))

(event `self.BuildingSpawnAnimation`
  (`parent.BuildingSpawnAnimation`)
  (`GameplayStatics.PlaySoundAtLocation` "/Game/Sound/Buildings/Resource_Tower_start_up.Resource_Tower_start_up" (`self.K2_GetActorLocation`) (struct) 1.0 1.0 0.0 null null null))

(event `self.InBackpack`
  (`parent.InBackpack`)
  (`KismetSystemLibrary.K2_PauseTimerHandle` (`self.TimerRef`)))

(event `self.Restored`
  (`parent.Restored`)
  (`KismetSystemLibrary.K2_UnPauseTimerHandle` (`self.TimerRef`)))

(event `self.CustomAnimation`
  (bind _rotatingshovelcomponent (`self.RotatingShovelComponent`))
  (bind (_direction _newtrack_0) (`Timeline|Timeline_1`)
    (:`Update`
      (`SceneComponent.K2_SetRelativeLocation` _rotatingshovelcomponent (`KismetMathLibrary.VLerp` (`SceneComponent.RelativeLocation` _rotatingshovelcomponent) (-60.0 48.0 -30.0) _newtrack_0) false false))
    (:`Finished`
      (`self.ShovelRotation`)
      (set `self.ShowUpgradeWidget` true)
      (`GameplayStatics.PlaySoundAtLocation` "/Game/Sound/Buildings/Resource_Tower_Loop.Resource_Tower_Loop" (`self.K2_GetActorLocation`) (struct) 1.0 1.0 0.0 null null null)
      (set `ParticleSystemComponent.CustomTimeDilation` 2.0 (`self.ParticleSystem`)))))

(fn `UserConstructionScript`
  (`parent.UserConstructionScript`))