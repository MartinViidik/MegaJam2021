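; Base building actor with an upgrade menu widget, backpack hide/restore and destruction events.
; On BeginPlay it fills the menu, spawns a cost popup and plays a timeline drop with sound, delayed camera shake and Niagara effects.
; The drop ends in an empty CustomAnimation hook.
; Upgrades check and deduct game mode money, show a popup, then raise cost and level and refresh the menu.
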(event `self.ReceiveBeginPlay`
  (bind _aswbp_upgrade_menu (cast `/Game/Blueprints/Widgets/WBP_UpgradeMenu` (`WidgetComponent.GetUserWidgetObject` (`self.UpgradeWidget`))))
  (bind _output_get (set `self.UpgradeMenu` _aswbp_upgrade_menu))
  (`/Game/Blueprints/Widgets/WBP_UpgradeMenu.UpdateUI` _output_get (`self.BuildingLvl`) (`self.BuildingTitle`) (`self.UpgradeCost`))
  (bind _returnvalue (`|SpawnActorFromClass` "/Game/Blueprints/Misc/Game/BP_ScoreUpdate.BP_ScoreUpdate_C" (`SceneComponent.K2_GetComponentToWorld` (`self.DefaultSceneRoot`)) "Undefined" "OverrideRootScale" null null))
  (`/Game/Blueprints/Misc/Game/BP_ScoreUpdate.UpdateText` _returnvalue (`self.BuildingCost`) false)
  (`self.BuildingSpawnAnimation`))

(event `SetWidgetVisibility`
  (params (bNewVisibility :type Boolean))
  (if (`self.ShowUpgradeWidget`)
    (`SceneComponent.SetVisibility` (`self.UpgradeWidget`) bNewVisibility false)))

(event `DestroyBuilding`
  (`self.K2_DestroyActor`))

(event `UpgradeBuilding`
  (bind _gamemode (`/Game/Blueprints/Functions/BP_Library.GetGameModeActor`))
  (bind _upgradecost (`self.UpgradeCost`))
  (if (>= (`/Game/Blueprints/Misc/Game/BP_GameMode.ReturnCurrentMoney` _gamemode) _upgradecost)
    (`/Game/Blueprints/Misc/Game/BP_GameMode.UpdateMoney` _gamemode (* _upgradecost -1))
    (bind _returnvalue (`|SpawnActorFromClass` "/Game/Blueprints/Misc/Game/BP_ScoreUpdate.BP_ScoreUpdate_C" (`SceneComponent.K2_GetComponentToWorld` (`self.DefaultSceneRoot`)) "Undefined" "OverrideRootScale" null null))
    (`/Game/Blueprints/Misc/Game/BP_ScoreUpdate.UpdateText` _returnvalue (`self.UpgradeCost`) false)
    (set `self.UpgradeCost` (+ (`self.UpgradeCost`) 50))
    (bind _result (`/Engine/EditorBlueprintResources/StandardMacros.IncrementInt` (`self.BuildingLvl`))
      (:`  `
        (set `self.BuildingLvl` _result)
        (`/Game/Blueprints/Widgets/WBP_UpgradeMenu.UpdateUI` (`self.UpgradeMenu`) (`self.BuildingLvl`) (`self.BuildingTitle`) (`self.UpgradeCost`))))))

(event `InBackpack`
  (`self.SetActorTickEnabled` false)
  (`self.SetActorHiddenInGame` true))

(event `Restored`
  (`self.SetActorTickEnabled` true)
  (`self.SetActorHiddenInGame` false))

(event `BuildingSpawnAnimation`
  (bind _defaultsceneroot (`self.DefaultSceneRoot`))
  (bind _relativelocation (`SceneComponent.RelativeLocation` (`self.DefaultSceneRoot`)))
  (`GameplayStatics.PlaySoundAtLocation` "/Game/Sound/Buildings/S_BuildingLand.S_BuildingLand" (`self.K2_GetActorLocation`) (struct) 1.0 1.0 0.0 null null null)
  (`self.StartShake`)
  (set `self.Relative Location` _relativelocation)
  (`SceneComponent.K2_SetRelativeLocation` (`self.DefaultSceneRoot`) (+ _relativelocation (0.0 0.0 500.0)) false false)
  (bind (_direction _newtrack_0) (`Timeline|Timeline_0`)
    (:`Update`
      (`SceneComponent.K2_SetRelativeLocation` _defaultsceneroot (`KismetMathLibrary.VLerp` (`SceneComponent.RelativeLocation` _defaultsceneroot) (`self.Relative Location`) _newtrack_0) false false))
    (:`Finished`
      (`NiagaraFunctionLibrary.SpawnSystemAtLocation` "/Game/VFX/BuildingBuildImpact/VFX_FallingBuilding1.VFX_FallingBuilding1" (`SceneComponent.K2_GetComponentLocation` (`self.DefaultSceneRoot`)) (struct) (1.0 1.0 1.0) true true "AutoRelease")
      (`self.CustomAnimation`))))

(event `CustomAnimation`)

(event `StartShake`
  (`KismetSystemLibrary.Delay` 0.3)
  (`MatineeCameraShake.StartMatineeCameraShake` (`GameplayStatics.GetPlayerCameraManager` 0) "/Game/Blueprints/Misc/CameraShake/BP_ExplosionShake.BP_ExplosionShake_C" 0.35 "World")
  (`NiagaraFunctionLibrary.SpawnSystemAtLocation` "/Game/VFX/BuildingBuildImpact/NewTry/NewNiagaraSystem.NewNiagaraSystem" (`self.K2_GetActorLocation`) (struct) (1.0 1.0 1.0) true true "AutoRelease"))

(fn `BuildingDestroyed`
  (`GameplayStatics.PlayWorldCameraShake` "/Game/Blueprints/Misc/CameraShake/BP_ExplosionShake.BP_ExplosionShake_C" (`self.K2_GetActorLocation`) 100.0 1000.0)
  (`self.K2_DestroyActor`))

(fn `UserConstructionScript`)