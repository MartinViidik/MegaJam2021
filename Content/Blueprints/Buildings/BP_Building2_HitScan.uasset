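; Hit-scan turret building, a child building Blueprint that damages targets with an instant line trace instead of firing projectiles.
; Damage is initialized from the projectile component's class defaults and increments on each upgrade, while actor tick is disabled.
; ShootProjectile traces forward from the spawn point, damaging living health components with muzzle, sound and shell-casing effects.
; A missed trace or invalid target makes the turret component search again.
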(event `/Game/Blueprints/Buildings/BP_BuildingBase.UpgradeBuilding`
  (`parent.UpgradeBuilding`)
  (`/Engine/EditorBlueprintResources/StandardMacros.IncrementInt` (`self.Damage`)))

(event `self.ReceiveBeginPlay`
  (`parent.ReceiveBeginPlay`)
  (`self.SetActorTickEnabled` false)
  (set `self.Damage` (defaults `Object` (`/Game/Blueprints/Components/BP_ProjectileComponent.ProjectileType` (`self.BP_ProjectileComponent`)))))

(event `self.ShootProjectile`
  (bind _shell1 (`self.Shell1`))
  (bind _shell2 (`self.Shell2`))
  (bind _spawnpoint00 (`self.SpawnPoint00`))
  (bind _bp_turretcomponent (`self.BP_TurretComponent`))
  (if (`self.IsActive`)
    (`/Engine/EditorBlueprintResources/StandardMacros.IsValid` (`/Game/Blueprints/Components/BP_TurretComponent.TargetActor` (`self.BP_TurretComponent`))
      (:`Is Valid`
        (bind (_out_hit_phys_mat _hit) (`/Game/Blueprints/Functions/BP_Library.LineTraceFunction` (`KismetMathLibrary.GetForwardVector` (`SceneComponent.K2_GetComponentRotation` (`self.SpawnPoint`))) self 2500.0))
        (if (`KismetSystemLibrary.IsValid` _hit)
          (bind _returnvalue (`self.GetComponentByClass` _hit "/Game/Blueprints/Components/BP_HealthComponent.BP_HealthComponent_C"))
          (`/Engine/EditorBlueprintResources/StandardMacros.IsValid` _returnvalue
            (:`Is Valid`
              (if (not (`/Game/Blueprints/Components/BP_HealthComponent.IsDead` _returnvalue))
                (`/Game/Blueprints/Components/BP_HealthComponent.UpdateHealth` _returnvalue (* (`self.Damage`) -1))
                (`NiagaraFunctionLibrary.SpawnSystemAttached` (`self.System Template Muzzle`) _spawnpoint00 "None" (0.0 0.0 0.0) (`SceneComponent.RelativeRotation` _spawnpoint00) "KeepRelativeOffset" false true "AutoRelease")
                (`GameplayStatics.PlaySoundAtLocation` "/Game/Sound/Weapons/GUN_TURRET_SHOT_Cue.GUN_TURRET_SHOT_Cue" (`self.K2_GetActorLocation`) (struct) 1.0 1.0 0.0 null null null)
                (`GameplayStatics.SpawnEmitterAtLocation` "/Game/VFX/Casings/PS_Casings.PS_Casings" (`SceneComponent.K2_GetComponentLocation` _shell1) (`KismetMathLibrary.Conv_VectorToRotator` (`SceneComponent.GetForwardVector` _shell1)) (1.0 1.0 1.0) true "AutoRelease")
                (`GameplayStatics.SpawnEmitterAtLocation` "/Game/VFX/Casings/PS_Casings.PS_Casings" (`SceneComponent.K2_GetComponentLocation` _shell2) (`KismetMathLibrary.Conv_VectorToRotator` (`SceneComponent.GetForwardVector` _shell2)) (1.0 1.0 1.0) true "AutoRelease"))))
          (else
            (set `/Game/Blueprints/Components/BP_TurretComponent.TargetActor` null _bp_turretcomponent)
            (`/Game/Blueprints/Components/BP_TurretComponent.SearchForTargets` _bp_turretcomponent))))
      (:`Is Not Valid`
        (`/Game/Blueprints/Components/BP_TurretComponent.SearchForTargets` (`self.BP_TurretComponent`))))))

(event `/Game/Blueprints/Buildings/BP_BuildingBase.CustomAnimation`
  (`parent.CustomAnimation`))

(event `/Game/Blueprints/Buildings/BP_BuildingBase.BuildingSpawnAnimation`
  (`parent.BuildingSpawnAnimation`))

(fn `UserConstructionScript`
  (`parent.UserConstructionScript`))