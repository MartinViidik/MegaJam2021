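; BP_Library is a Blueprint function library of small shared helpers for actor directions, game mode access and line tracing.
; GetUpVector and GetForwardVector both return the up vector of an actor's rotation, despite the latter's name.
; GetGameModeActor returns the game mode cast to BP_GameMode.
; LineTraceFunction traces the Visibility channel from an actor's location along a given direction and length, draws debug lines, and returns any blocking hit actor.
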(fn `GetForwardVector`
  (params (Target :type "Actor Object Reference"))
  (returns (Vector :type "Vector Structure"))
  (return (`KismetMathLibrary.GetUpVector` (`Actor.K2_GetActorRotation` Target))))

(fn `GetGameModeActor`
  (returns (GameMode :type "/Game/Blueprints/Misc/Game/BP_GameMode Object Reference"))
  (bind _asbp_game_mode (cast `/Game/Blueprints/Misc/Game/BP_GameMode` (`GameplayStatics.GetGameMode` (`local.__WorldContext`))))
  (return _asbp_game_mode))

(fn `GetUpVector`
  (params (NewParam :type "Actor Object Reference"))
  (returns (Vector :type "Vector Structure"))
  (return (`KismetMathLibrary.GetUpVector` (`Actor.K2_GetActorRotation` NewParam))))

(fn `LineTraceFunction`
  (params (Direction :type "Vector Structure") (Actor :type "Actor Object Reference") (Length :type "Float (double-precision)"))
  (returns (Hit :type "Actor Object Reference"))
  (bind _returnvalue (`Actor.K2_GetActorLocation` Actor))
  (bind _outhit (`KismetSystemLibrary.LineTraceSingle` :`Start` _returnvalue :`End` (+ _returnvalue (* Direction Length)) :`TraceChannel` "TraceTypeQuery1" :`DrawDebugType` "ForDuration"))
  (if (`GameplayStatics.BreakHitResult` _outhit)
    (return (`.HitActor` (`GameplayStatics.BreakHitResult` _outhit)))))